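; A hand laser pointer actor that draws a blue Niagara beam along its forward vector.
; On BeginPlay it colors both effects and caches the BP_SJ_OutOfZone actor so traces ignore it.
; Each Tick it line-traces on the Camera channel up to Distance, setting the beam's LaserEnd to the hit point or trace end.
; The impact effect moves to the hit location and shows only on a blocking hit.
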(event `self.ReceiveBeginPlay`
  (`FXSystemComponent.SetColorParameter` (`self.NiagaraLaser`) "Color" (struct :`G` 0.436092 :`B` 1.0 :`A` 1.0))
  (`FXSystemComponent.SetColorParameter` (`self.NiagaraLaserImpact`) "Color" (struct :`G` 0.436092 :`B` 1.0 :`A` 1.0))
  (bind _returnvalue (`GameplayStatics.GetActorOfClass` "/Game/SJ/Blueprints/PingPong/PingPongTable/BP_SJ_OutOfZone.BP_SJ_OutOfZone_C")))

(event `self.ReceiveTick`
  (params (DeltaSeconds :type "Float (single-precision)"))
  (bind _returnvalue (`self.K2_GetActorLocation`))
  (bind _returnvalue_2 (+ _returnvalue (* (`self.GetActorForwardVector`) (`self.Distance`))))
  ;[1 1 1] 라인 트레이스 끝 부분 구하기
  (set `self.TraceEnd` _returnvalue_2)
  (bind _outhit (`KismetSystemLibrary.LineTraceSingle` _returnvalue _returnvalue_2 "TraceTypeQuery2" false (`|MakeArray` (stale `self.ReceiveBeginPlay` _returnvalue) :!type "Actor Object Reference")))
  (set `self.Hit` (`GameplayStatics.BreakHitResult` _outhit))
  ;[1 1 1] 라인이 충돌한 위치
  (set `self.HitLocation` (`.Location` (`GameplayStatics.BreakHitResult` _outhit)))
  ;[1 1 1] LaserEnd 나이아가라 시스템의 변수 새로 할당하기
  (`FXSystemComponent.SetVectorParameter` (`self.NiagaraLaser`) "LaserEnd" (select `bool` (`self.Hit`) :`false` (`self.TraceEnd`) :`true` (`self.HitLocation`)))
  ;[1 1 1] 부딪힌 지점이 있다면 임팩트 파티클 활성화
  (`SceneComponent.SetVisibility` (`self.NiagaraLaserImpact`) (`self.Hit`) false)
  ;[1 1 1] 부딪힌 지점으로 임팩트 파티클 옮기기
  (`SceneComponent.K2_SetWorldLocation` (`self.NiagaraLaserImpact`) (`self.HitLocation`) false false))

(fn `UserConstructionScript`)