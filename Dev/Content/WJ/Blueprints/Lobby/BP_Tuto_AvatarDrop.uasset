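; Lobby tutorial actor, named for avatar drop, that animates its Move component in an endless back-and-forth motion.
; Each Tick lerps the component's relative location toward one of two fixed points on a Y-Z diagonal, flipping the Down flag when within a small distance.
; Lerping from the current position eases each swing to a stop and makes the speed frame-rate dependent, as delta time is unused.
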(event `self.ReceiveTick`
  (params (DeltaSeconds :type "Float (single-precision)"))
  (bind _alpha (`self.Alpha`))
  (bind _move (`self.Move`))
  (bind _relativelocation (`SceneComponent.RelativeLocation` _move))
  (if (`self.bDown`)
    (`SceneComponent.K2_SetRelativeLocation` _move (`KismetMathLibrary.VLerp` _relativelocation (0.0 30.0 30.0) _alpha) false false)
    (if (<= (`KismetMathLibrary.Vector_Distance` _relativelocation (0.0 30.0 30.0)) 2.0)
      (set `self.bDown` false))
    (else
      (`SceneComponent.K2_SetRelativeLocation` _move (`KismetMathLibrary.VLerp` _relativelocation (0.0 -24.0 -24.0) _alpha) false false)
      (if (<= (`KismetMathLibrary.Vector_Distance` _relativelocation (0.0 -24.0 -24.0)) 2.0)
        (set `self.bDown` true)))))

(fn `UserConstructionScript`)